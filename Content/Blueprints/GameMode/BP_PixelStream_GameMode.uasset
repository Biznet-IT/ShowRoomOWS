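; Game mode for a Pixel Streaming app that sets up players, LAN sessions and browser input.
; PostLogin spawns and possesses a third-person character, creating another orbit controller when the controller list exceeds one, then joins or creates a session.
; New streaming connections record player IDs on orbit controllers.
; Browser JSON events route config, zoom and resolution changes to player 0's orbit controller, and encoder, frame-rate and bitrate settings to console commands.
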(event Custom|OnNewConnection_Event_0
  (params (StreamerId :type String) (PlayerId :type String) (QualityController :type Boolean))
  (bind _thisplayer (Variables|MyGame|GetThisPlayer))
  ;[1 1 1] Begin Play
  (if (== _thisplayer "/Game/Blueprints/Pawn/BP_Orbit_Controller.BP_Orbit_Controller")
    (bind _output_get (Variables|MyGame|SetMyPlayerId PlayerId))
    (Utilities|Array|Add (Variables|/Game/Blueprints/Pawn/BP_Orbit_Controller.BP_Orbit_Controller_C|GetPlayersIds _thisplayer) _output_get)
    (else
      (bind _output_get_2 (Variables|MyGame|SetMyPlayerId PlayerId))
      (bind _asbp_orbit_controller (Utilities|Casting|CastToBP_Orbit_Controller (Game|GetPlayerController 0)))
      (Utilities|Array|Add (Variables|/Game/Blueprints/Pawn/BP_Orbit_Controller.BP_Orbit_Controller_C|GetPlayersIds _asbp_orbit_controller) _output_get_2))))

(event Custom|OnJSONEvent
  (params (Descriptor :type String))
  ;[1 1 1] Bind JSON events - This is listening for HTML/JavaScript events from the Pixel Streaming client's web browser.
  (bind _output_get (Variables|/Game/Blueprints/Pawn/BP_Orbit_Controller.BP_Orbit_Controller_C|SetDescriptor (Variables|MyGame|GetThisPlayer) Descriptor))
  (Variables|Default|SetDescriptor _output_get)
  (bind _asbp_orbit_controller (Utilities|Casting|CastToBP_Orbit_Controller (Game|GetPlayerController 0)))
  (if (.Success (Class|PixelStreamingInput|GetJsonStringValue (Variables|Default|GetPixelStreamingInput) (Variables|Default|GetDescriptor) "Category"))
    (Default|ChangeConfigOption _asbp_orbit_controller)
    (elif (.Success (Class|PixelStreamingInput|GetJsonStringValue (Variables|Default|GetPixelStreamingInput) (Variables|Default|GetDescriptor) "Zoom"))
      (Default|ToggleZoom _asbp_orbit_controller)
      (elif (.Success (Class|PixelStreamingInput|GetJsonStringValue (Variables|Default|GetPixelStreamingInput) (Variables|Default|GetDescriptor) "Resolution"))
        (Default|ChangeResolution _asbp_orbit_controller)
        (elif (.Success (Class|PixelStreamingInput|GetJsonStringValue (Variables|Default|GetPixelStreamingInput) (Variables|Default|GetDescriptor) "MaxQP"))
          (Development|ExecuteConsoleCommand (Utilities|String|Append "PixelStreaming.Encoder.MaxQP " (.StringValue (Class|PixelStreamingInput|GetJsonStringValue (Variables|Default|GetPixelStreamingInput) (Variables|Default|GetDescriptor) "MaxQP"))) _asbp_orbit_controller)
          (elif (.Success (Class|PixelStreamingInput|GetJsonStringValue (Variables|Default|GetPixelStreamingInput) (Variables|Default|GetDescriptor) "MinQP"))
            (Development|ExecuteConsoleCommand (Utilities|String|Append "PixelStreaming.Encoder.MinQP " (.StringValue (Class|PixelStreamingInput|GetJsonStringValue (Variables|Default|GetPixelStreamingInput) (Variables|Default|GetDescriptor) "MinQP"))) _asbp_orbit_controller)
            (elif (.Success (Class|PixelStreamingInput|GetJsonStringValue (Variables|Default|GetPixelStreamingInput) (Variables|Default|GetDescriptor) "MaxFPS"))
              (Development|ExecuteConsoleCommand (Utilities|String|Append "t.MaxFPS " (.StringValue (Class|PixelStreamingInput|GetJsonStringValue (Variables|Default|GetPixelStreamingInput) (Variables|Default|GetDescriptor) "MaxFPS"))) _asbp_orbit_controller)
              (elif (.Success (Class|PixelStreamingInput|GetJsonStringValue (Variables|Default|GetPixelStreamingInput) (Variables|Default|GetDescriptor) "MaxBitrate"))
                (Development|ExecuteConsoleCommand (Utilities|String|Append "PixelStreaming.WebRTC.MaxBitrate " (.StringValue (Class|PixelStreamingInput|GetJsonStringValue (Variables|Default|GetPixelStreamingInput) (Variables|Default|GetDescriptor) "MaxBitrate"))) _asbp_orbit_controller)))))))))

(event EventPostLogin
  (params (NewPlayer :type Player%20Controller%20Object%20Reference))
  (bind _initial_location (Variables|Default|GetInitial%20Location))
  ;[1 1 1] Server - Client Logic
  (bind _asbp_orbit_controller (Utilities|Casting|CastToBP_Orbit_Controller NewPlayer))
  (bind _output_get (Variables|MyGame|SetThisPlayer _asbp_orbit_controller))
  (Utilities|Array|Add (Variables|/Game/Blueprints/Pawn/BP_Orbit_Controller.BP_Orbit_Controller_C|GetPlayerControllers _asbp_orbit_controller) _output_get)
  (if (== 1 (Utilities|Array|Length (Variables|/Game/Blueprints/Pawn/BP_Orbit_Controller.BP_Orbit_Controller_C|GetPlayerControllers _asbp_orbit_controller)))
    (bind _returnvalue (Game|SpawnActorfromClass "/Game/ThirdPerson/Blueprints/BP_ThirdPersonCharacter.BP_ThirdPersonCharacter_C" _initial_location "AlwaysSpawn" _output_get 0))
    (Pawn|UnPossess _asbp_orbit_controller)
    (Pawn|Possess _output_get _returnvalue)
    (else
      (bind _returnvalue_2 (Game|SpawnActorfromClass "/Game/Blueprints/Pawn/BP_Orbit_Controller.BP_Orbit_Controller_C" _initial_location "Undefined" 0 0 0))
      (Utilities|Array|Add (Variables|/Game/Blueprints/Pawn/BP_Orbit_Controller.BP_Orbit_Controller_C|GetPlayerControllers _asbp_orbit_controller) _returnvalue_2)
      (bind _output_get_2 (Variables|MyGame|SetThisPlayer _returnvalue_2))
      (bind _returnvalue_3 (Game|SpawnActorfromClass "/Game/ThirdPerson/Blueprints/BP_ThirdPersonCharacter.BP_ThirdPersonCharacter_C" _initial_location "Undefined" _returnvalue_2 0))
      (Pawn|UnPossess _output_get_2)
      (Pawn|Possess _output_get_2 _returnvalue_3)))
  (if (== 1 (Utilities|Array|Length (Variables|/Game/Blueprints/Pawn/BP_Orbit_Controller.BP_Orbit_Controller_C|GetPlayerControllers _asbp_orbit_controller)))
    (Variables|MyGame|SetIsServer? true)
    (else
      (Variables|MyGame|SetIsServer? false)))
  (Variables|Default|SetTotal%20Players (Utilities|Array|Length (Variables|/Game/Blueprints/Pawn/BP_Orbit_Controller.BP_Orbit_Controller_C|GetPlayerControllers _asbp_orbit_controller)))
  (bind _results (|FindSessions _output_get_2 1 true)
    (:OnSuccess
      (|JoinSession 0 (Utilities|Array|Get(acopy) _results)))
    (:OnFailure
      (|Session _output_get_2 100 true))))

(event EventBeginPlay
  ;[1 1 1] Begin Play
  (EventDispatchers|BindEventtoOnInputEvent (Variables|Default|GetPixelStreamingInput) (delegate Custom|OnJSONEvent))
  (bind _returnvalue (Class|PixelStreamingBlueprints|GetPixelStreamingDelegates))
  (EventDispatchers|AssignOnNewConnection _returnvalue (delegate Custom|OnNewConnection_Event_0)))

(fn ConstructionScript)

(fn OnRepThisPlayer)

(fn OnRepMyPlayerId)

(fn OnRepIsServer?)

(fn GetDefaultPawnClassforController
  (params (InController :type Controller%20Object%20Reference))
  (return (Utilities|GetClass InController)))

(fn OnRepPlayersControllers)

(fn ChoosePlayerStart
  (params (Player :type Controller%20Object%20Reference))
  (bind _outactors (Actor|GetAllActorsOfClass "/Script/Engine.PlayerStart"))
  (Actor|SetOwner (Utilities|Array|Get(acopy) _outactors) Player)
  (return (Utilities|Array|Get(acopy) _outactors)))

(fn FindPlayerStart
  (params (Player :type Controller%20Object%20Reference) (IncomingName :type String))
  (bind _outactors (Actor|GetAllActorsOfClass "/Script/Engine.PlayerStart"))
  (Actor|SetOwner (Utilities|Array|Get(acopy) _outactors) Player)
  (return (Utilities|Array|Get(acopy) _outactors)))