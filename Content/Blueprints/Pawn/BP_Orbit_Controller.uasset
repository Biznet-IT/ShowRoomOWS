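; Orbit controller for a Pixel Streaming character configurator, turning JSON descriptors from the web page into scene changes.
; A Category field routes to character or skin changes on the level's BP_CharConfig, or to environment and time-of-day changes.
; Ruins/Fortress and day/night swaps toggle streaming level visibility behind camera fades, with F and R as keyboard shortcuts.
; Other events toggle the third-person pawn's zoom and set resolution by console command.
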(event Custom|ToggleZoom
  (bind _playerpawn (Variables|Default|GetPlayerPawn))
  (bind _descriptor (Variables|Default|GetDescriptor))
  (bind _pixelstreaminginput (Variables|Default|GetPixelStreamingInput))
  (bind (_stringvalue _success) (Class|PixelStreamingInput|GetJsonStringValue _pixelstreaminginput _descriptor "Zoom"))
  ;[1 1 1] JSON Event: Toggle Zoom
  (if _success
    (switch string _stringvalue
      (:1
        (Utilities|FlowControl|FlipFlop
          (:A
            (Variables|/Game/ThirdPerson/Blueprints/BP_ThirdPersonCharacter.BP_ThirdPersonCharacter_C|SetTarget%20Zoom _playerpawn 1.2e+02))
          (:B
            (Variables|/Game/ThirdPerson/Blueprints/BP_ThirdPersonCharacter.BP_ThirdPersonCharacter_C|SetTarget%20Zoom _playerpawn 5e+02)))))))

(event Custom|ChangeResolution
  (bind _descriptor (Variables|Default|GetDescriptor))
  (bind _pixelstreaminginput (Variables|Default|GetPixelStreamingInput))
  (bind _descriptor_2 (Variables|Default|GetDescriptor))
  (bind _pixelstreaminginput_2 (Variables|Default|GetPixelStreamingInput))
  (bind (_stringvalue _success) (Class|PixelStreamingInput|GetJsonStringValue _pixelstreaminginput _descriptor "X"))
  (bind (_stringvalue_2 _success_2) (Class|PixelStreamingInput|GetJsonStringValue _pixelstreaminginput_2 _descriptor_2 "Y"))
  ;[1 1 1] JSON Event: Resolution
  (if _success
    (if _success_2
      (Development|ExecuteConsoleCommand (Utilities|String|Append "r.setres " _stringvalue "x" _stringvalue_2) 0))))

(event Custom|ChangeCharacter
  (bind _descriptor (Variables|Default|GetDescriptor))
  (bind _pixelstreaminginput (Variables|Default|GetPixelStreamingInput))
  (bind _stringvalue (Class|PixelStreamingInput|GetJsonStringValue _pixelstreaminginput _descriptor "Item"))
  ;[1 1 1] Change Character
  (if true
    (Development|PrintString _stringvalue true true "(R=1.000000,G=0.409627,B=0.000000,A=1.000000)" 2e+01)
    (Default|ChangeCharacter (Variables|Default|GetCharConfigRef) (Math|Conversions|ToInteger(Byte) _stringvalue))))

(event Custom|ChangeEnv
  (bind _pixelstreaminginput (Variables|Default|GetPixelStreamingInput))
  (bind _descriptor (Variables|Default|GetDescriptor))
  (bind (_stringvalue _success) (Class|PixelStreamingInput|GetJsonStringValue _pixelstreaminginput _descriptor "Item"))
  ;[1 1 1] Change Env
  (if _success
    (Variables|Default|SetMapSelection _stringvalue)
    (CameraFades|StartCameraFade :self (Game|GetPlayerCameraManager 0) :ToAlpha 1.0 :Duration 0.5 :bShouldFadeAudio true :bHoldWhenFinished true)
    (Utilities|FlowControl|Delay 0.7)
    (Variables|/Script/Engine.LevelStreaming|SetbShouldBeVisible (Class|GameplayStatics|GetStreamingLevel "Fortress_Base") (Utilities|Enum|Equal(Enum) (Variables|Default|GetMapSelection) "1"))
    (Variables|/Script/Engine.LevelStreaming|SetbShouldBeVisible (Class|GameplayStatics|GetStreamingLevel "Ruins_Daylight") false)
    (Variables|/Script/Engine.LevelStreaming|SetbShouldBeVisible (Class|GameplayStatics|GetStreamingLevel "Ruins_Night") false)
    (Variables|/Script/Engine.LevelStreaming|SetbShouldBeVisible (Class|GameplayStatics|GetStreamingLevel "Ruins_Base") (Utilities|Enum|Equal(Enum) (Variables|Default|GetMapSelection) "0"))
    (Variables|/Script/Engine.LevelStreaming|SetbShouldBeVisible (Class|GameplayStatics|GetStreamingLevel "Fortress_Daylight") false)
    (Variables|/Script/Engine.LevelStreaming|SetbShouldBeVisible (Class|GameplayStatics|GetStreamingLevel "Fortress_Night") false)
    (CallFunction|ChangeTime true)))

(event Custom|ChangeSkin
  (bind _descriptor (Variables|Default|GetDescriptor))
  (bind _pixelstreaminginput (Variables|Default|GetPixelStreamingInput))
  (bind (_stringvalue _success) (Class|PixelStreamingInput|GetJsonStringValue _pixelstreaminginput _descriptor "Item"))
  ;[1 1 1] Change Skin
  (if _success
    (Default|ChangeSkin (Variables|Default|GetCharConfigRef) (Math|Conversions|ToInteger(Byte) _stringvalue))))

(event Custom|ChangeTime
  (params (BypassHTML :type Boolean))
  (bind _descriptor (Variables|Default|GetDescriptor))
  (bind _pixelstreaminginput (Variables|Default|GetPixelStreamingInput))
  (bind (_stringvalue _success) (Class|PixelStreamingInput|GetJsonStringValue _pixelstreaminginput _descriptor "Item"))
  ;[1 1 1] Change Time of Day
  (if BypassHTML
    (switch string (Variables|Default|GetMapSelection) :!label _label
      (:0
        (switch string (Variables|Default|GetCurrentTime)
          (:0
            (Variables|/Script/Engine.LevelStreaming|SetbShouldBeVisible (Class|GameplayStatics|GetStreamingLevel "Ruins_Daylight") true)
            (Variables|/Script/Engine.LevelStreaming|SetbShouldBeVisible (Class|GameplayStatics|GetStreamingLevel "Ruins_Night") false))
          (:1
            (Variables|/Script/Engine.LevelStreaming|SetbShouldBeVisible (Class|GameplayStatics|GetStreamingLevel "Ruins_Daylight") false)
            (Variables|/Script/Engine.LevelStreaming|SetbShouldBeVisible (Class|GameplayStatics|GetStreamingLevel "Ruins_Night") true))))
      (:1
        (switch string (Variables|Default|GetCurrentTime)
          (:0
            (Variables|/Script/Engine.LevelStreaming|SetbShouldBeVisible (Class|GameplayStatics|GetStreamingLevel "Fortress_Daylight") true)
            (Variables|/Script/Engine.LevelStreaming|SetbShouldBeVisible (Class|GameplayStatics|GetStreamingLevel "Fortress_Night") false))
          (:1
            (Variables|/Script/Engine.LevelStreaming|SetbShouldBeVisible (Class|GameplayStatics|GetStreamingLevel "Fortress_Daylight") false)
            (Variables|/Script/Engine.LevelStreaming|SetbShouldBeVisible (Class|GameplayStatics|GetStreamingLevel "Fortress_Night") true)))))
    (Utilities|FlowControl|Delay 0.5)
    (CameraFades|StartCameraFade :self (Game|GetPlayerCameraManager 0) :FromAlpha 1.0 :Duration 0.5 :bShouldFadeAudio true)
    (elif _success
      (Variables|Default|SetCurrentTime _stringvalue)
      (CameraFades|StartCameraFade :self (Game|GetPlayerCameraManager 0) :ToAlpha 1.0 :Duration 0.5 :bShouldFadeAudio true :bHoldWhenFinished true)
      (Utilities|FlowControl|Delay 0.7)
      (goto _label))))

(event Custom|ChangeConfigOption
  (bind _descriptor (Variables|Default|GetDescriptor))
  (bind _pixelstreaminginput (Variables|Default|GetPixelStreamingInput))
  (bind (_stringvalue _success) (Class|PixelStreamingInput|GetJsonStringValue _pixelstreaminginput _descriptor "Category"))
  ;[1 1 1] JSON Event: Change Config Option
  (if _success
    (switch string _stringvalue
      (:0
        (CallFunction|ChangeCharacter))
      (:1
        (CallFunction|ChangeSkin))
      (:2
        (CallFunction|ChangeEnv))
      (:3
        (CallFunction|ChangeTime false)))))

(event EventBeginPlay
  ;[1 1 1] Begin Play
  (bind _asbp_third_person_character (Utilities|Casting|CastToBP_ThirdPersonCharacter (Game|Player|GetPlayerPawn 0))
    (:then
      (bind _output_get (Variables|Default|SetPlayerPawn _asbp_third_person_character))
      (Utilities|Array|Add (Variables|Default|GetPlayerPawns) _output_get)
      (bind _outactors (Actor|GetAllActorsOfClass "/Game/Blueprints/CharacterConfig/BP_CharConfig.BP_CharConfig_C"))
      (for _array_element _outactors
        (Variables|Default|SetCharConfigRef _array_element)))
    (:CastFailed
      (Development|PrintString "Not Working, wait" true true "(R=1.000000,G=0.000000,B=0.011645,A=1.000000)" 15.0))))

(event Input|KeyboardEvents|R
  (params (Key :type Key%20Structure))
  ;[1 1 1] Change Time of Day
  (:Pressed
    (Utilities|FlowControl|FlipFlop
      (:A
        (Variables|Default|SetCurrentTime "1"))
      (:B
        (Variables|Default|SetCurrentTime "0")))
    (CameraFades|StartCameraFade :self (Game|GetPlayerCameraManager 0) :ToAlpha 1.0 :Duration 0.5 :bShouldFadeAudio true :bHoldWhenFinished true)
    (Utilities|FlowControl|Delay 0.7)
    (switch string (Variables|Default|GetMapSelection)
      (:0
        (switch string (Variables|Default|GetCurrentTime)
          (:0
            (Variables|/Script/Engine.LevelStreaming|SetbShouldBeVisible (Class|GameplayStatics|GetStreamingLevel "Ruins_Daylight") true)
            (Variables|/Script/Engine.LevelStreaming|SetbShouldBeVisible (Class|GameplayStatics|GetStreamingLevel "Ruins_Night") false))
          (:1
            (Variables|/Script/Engine.LevelStreaming|SetbShouldBeVisible (Class|GameplayStatics|GetStreamingLevel "Ruins_Daylight") false)
            (Variables|/Script/Engine.LevelStreaming|SetbShouldBeVisible (Class|GameplayStatics|GetStreamingLevel "Ruins_Night") true))))
      (:1
        (switch string (Variables|Default|GetCurrentTime)
          (:0
            (Variables|/Script/Engine.LevelStreaming|SetbShouldBeVisible (Class|GameplayStatics|GetStreamingLevel "Fortress_Daylight") true)
            (Variables|/Script/Engine.LevelStreaming|SetbShouldBeVisible (Class|GameplayStatics|GetStreamingLevel "Fortress_Night") false))
          (:1
            (Variables|/Script/Engine.LevelStreaming|SetbShouldBeVisible (Class|GameplayStatics|GetStreamingLevel "Fortress_Daylight") false)
            (Variables|/Script/Engine.LevelStreaming|SetbShouldBeVisible (Class|GameplayStatics|GetStreamingLevel "Fortress_Night") true)))))
    (Utilities|FlowControl|Delay 0.5)
    (CameraFades|StartCameraFade :self (Game|GetPlayerCameraManager 0) :FromAlpha 1.0 :Duration 0.5 :bShouldFadeAudio true)))

(event Input|KeyboardEvents|F
  (params (Key :type Key%20Structure))
  ;[1 1 1] Change Env
  (:Pressed
    (Utilities|FlowControl|FlipFlop
      (:A
        (Variables|Default|SetMapSelection "1"))
      (:B
        (Variables|Default|SetMapSelection "0")))
    (CameraFades|StartCameraFade :self (Game|GetPlayerCameraManager 0) :ToAlpha 1.0 :Duration 0.5 :bShouldFadeAudio true :bHoldWhenFinished true)
    (Utilities|FlowControl|Delay 0.7)
    (Variables|/Script/Engine.LevelStreaming|SetbShouldBeVisible (Class|GameplayStatics|GetStreamingLevel "Fortress_Base") (Utilities|Enum|Equal(Enum) (Variables|Default|GetMapSelection) "1"))
    (Variables|/Script/Engine.LevelStreaming|SetbShouldBeVisible (Class|GameplayStatics|GetStreamingLevel "Ruins_Daylight") false)
    (Variables|/Script/Engine.LevelStreaming|SetbShouldBeVisible (Class|GameplayStatics|GetStreamingLevel "Ruins_Night") false)
    (Variables|/Script/Engine.LevelStreaming|SetbShouldBeVisible (Class|GameplayStatics|GetStreamingLevel "Ruins_Base") (Utilities|Enum|Equal(Enum) (Variables|Default|GetMapSelection) "0"))
    (Variables|/Script/Engine.LevelStreaming|SetbShouldBeVisible (Class|GameplayStatics|GetStreamingLevel "Fortress_Daylight") false)
    (Variables|/Script/Engine.LevelStreaming|SetbShouldBeVisible (Class|GameplayStatics|GetStreamingLevel "Fortress_Night") false)
    (CallFunction|ChangeTime true)))

(fn ConstructionScript)

(fn OnRepPlayerControllers)

(fn OnRepPLayersId)