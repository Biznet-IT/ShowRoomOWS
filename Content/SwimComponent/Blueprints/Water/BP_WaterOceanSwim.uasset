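; BP_WaterOceanSwim is an ocean water body that acts as a swim volume for the Swim component.
; Overlap begin and end send enter and exit water volume messages to the other actor, passing itself.
; GetWaterVolumeInfo reports it as UE Water System water with buoyancy helper allowed, taking surface height from the spline's world Z alongside an offset and swim priority.
; The surface height is flagged as not needing updates.
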(event EventBeginPlay)

(event Collision|EventActorBeginOverlap
  (params (OtherActor :type Actor%20Object%20Reference))
  ;[0.0616 0.3004 1] These events serve the Swim component
  (Class|BPISwim|EnterWaterVolume(Message) OtherActor self))

(event EventTick
  (params (DeltaSeconds :type Float%20%28single-precision%29)))

(event Collision|EventActorEndOverlap
  (params (OtherActor :type Actor%20Object%20Reference))
  ;[0.0616 0.3004 1] These events serve the Swim component
  (Class|BPISwim|ExitWaterVolume(Message) OtherActor self))

(fn ConstructionScript)

(fn GetSwimComponent
  (return 0))

(fn GetWaterVolumeInfo
  (params (Player :type Actor%20Object%20Reference))
  (return (.z (Transformation|GetWorldLocation (Variables|Default|GetSplineComp))) true true false (Variables|Default|GetPrioritySwim) (Variables|Default|GetOffsetZLocation) true false))