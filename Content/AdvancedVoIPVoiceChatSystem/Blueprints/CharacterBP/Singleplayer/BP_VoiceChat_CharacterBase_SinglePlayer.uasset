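; Single-player voice chat character base that sends captured player audio to radio actors while the positional voice input is held, marked as a test example.
; BeginPlay caches every BP_VoiceActor_Radio tagged VOIPoutput.
; Pressing the input runs ToggleSpeaking 1 and passes AudioCaptureUsedForSinglePlayer to each cached radio, while release or cancel reverses both.
; An inline note explains how submix and bus send settings govern echo playback and spectrum analysis.
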(event Input|EnhancedActionEvents|EnhancedInputActionIA_VoiceChat_Positional
  (params (ActionValue :type Boolean) (ElapsedSeconds :type Float%20%28double-precision%29) (TriggeredSeconds :type Float%20%28double-precision%29) (InputAction :type Input%20Action%20Object%20Reference :default "/Game/AdvancedVoIPVoiceChatSystem/Input/Actions/IA_VoiceChat_Positional.IA_VoiceChat_Positional"))
  ;[1 1 1] #TEST - Example
  (:Started
    (Development|ExecuteConsoleCommand "ToggleSpeaking 1" 0)
    (for _array_element (Variables|Default|GetOut%20Actors%20Radio%20List)
      (Default|SentSubmittoRadio _array_element (Variables|Default|GetAudioCaptureUsedForSinglePlayer))))
  (:Canceled
    (Development|ExecuteConsoleCommand "ToggleSpeaking 0" 0 :!label _label)
    (for _array_element_2 (Variables|Default|GetOut%20Actors%20Radio%20List)
      (Default|StopSubmittoRadio _array_element_2 (Variables|Default|GetAudioCaptureUsedForSinglePlayer))))
  (:Completed
    (goto _label)))

(event EventBeginPlay
  (bind _outactors (Actor|GetAllActorsOfClasswithTag "/Game/AdvancedVoIPVoiceChatSystem/Blueprints/VoiceActors/BP_VoiceActor_Radio.BP_VoiceActor_Radio_C" "VOIPoutput"))
  (Variables|Default|SetOut%20Actors%20Radio%20List _outactors))

(fn ConstructionScript
  (|CallParentFunction))