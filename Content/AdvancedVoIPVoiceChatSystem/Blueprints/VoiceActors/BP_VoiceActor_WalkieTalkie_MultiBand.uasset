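; Walkie-talkie voice actor for multi-band radio in the voice chat system, handling receiver audio on three selectable frequencies.
; Both receiver events run one check: when the radio is on, the replicated frequency picks the sounds for the main audio and five signal-jammer components.
; When off, it deactivates those plus beep and static components, whose activation calls are unwired.
; Interface functions return a self reference, and the frequency OnRep is empty.
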(event EventBeginPlay
  (|CallParentFunction))

(event EventDeactivateReceiverOutput
  (bind _signaljammer_m (Variables|Default|GetSignalJammer_M))
  (bind _signaljammer_l (Variables|Default|GetSignalJammer_L))
  (bind _signaljammer_m1 (Variables|Default|GetSignalJammer_M1))
  (bind _signaljammer_h (Variables|Default|GetSignalJammer_H))
  (bind _signaljammer_c (Variables|Default|GetSignalJammer_C))
  (bind _audio (Variables|Default|GetAudio))
  (if (Variables|Default|GetisWalkieTalkieOn?)
    (switch Utilities|FlowControl|Switch|SwitchonE_RadioFrequencies (Variables|Default|GetFrequencies)
      (:NewEnumerator0
        (Audio|Components|Audio|SetSound _audio "/Game/AdvancedVoIPVoiceChatSystem/Audio/Radio_Buses/SB_radioSourceBus_99_1.SB_radioSourceBus_99_1")
        (Components|Activation|Activate _audio false)
        (Audio|Components|Audio|SetSound _signaljammer_l "/Game/AdvancedVoIPVoiceChatSystem/Audio/Radio_Buses/PlayersBoxes/SB_99_1L.SB_99_1L")
        (Components|Activation|Activate _signaljammer_l false)
        (Audio|Components|Audio|SetSound _signaljammer_m "/Game/AdvancedVoIPVoiceChatSystem/Audio/Radio_Buses/PlayersBoxes/SB_99_1M.SB_99_1M")
        (Components|Activation|Activate _signaljammer_m false)
        (Audio|Components|Audio|SetSound _signaljammer_m1 "/Game/AdvancedVoIPVoiceChatSystem/Audio/Radio_Buses/PlayersBoxes/SB_99_1M1.SB_99_1M1")
        (Components|Activation|Activate _signaljammer_m1 false)
        (Audio|Components|Audio|SetSound _signaljammer_h "/Game/AdvancedVoIPVoiceChatSystem/Audio/Radio_Buses/PlayersBoxes/SB_99_1H.SB_99_1H")
        (Components|Activation|Activate _signaljammer_h false)
        (Audio|Components|Audio|SetSound _signaljammer_c "/Game/AdvancedVoIPVoiceChatSystem/Audio/Radio_Buses/PlayersBoxes/SB_99_1C.SB_99_1C")
        (Components|Activation|Activate _signaljammer_c false)
        (Development|PrintString "99"))
      (:NewEnumerator1
        (Audio|Components|Audio|SetSound _audio "/Game/AdvancedVoIPVoiceChatSystem/Audio/Radio_Buses/SB_radioSourceBus_102_6.SB_radioSourceBus_102_6")
        (Components|Activation|Activate _audio false)
        (Audio|Components|Audio|SetSound _signaljammer_l "/Game/AdvancedVoIPVoiceChatSystem/Audio/Radio_Buses/PlayersBoxes/SB_102_6L.SB_102_6L")
        (Components|Activation|Activate _signaljammer_l false)
        (Audio|Components|Audio|SetSound _signaljammer_m "/Game/AdvancedVoIPVoiceChatSystem/Audio/Radio_Buses/PlayersBoxes/SB_102_6M.SB_102_6M")
        (Components|Activation|Activate _signaljammer_m false)
        (Audio|Components|Audio|SetSound _signaljammer_m1 "/Game/AdvancedVoIPVoiceChatSystem/Audio/Radio_Buses/PlayersBoxes/SB_102_6M1.SB_102_6M1")
        (Components|Activation|Activate _signaljammer_m1 false)
        (Audio|Components|Audio|SetSound _signaljammer_h "/Game/AdvancedVoIPVoiceChatSystem/Audio/Radio_Buses/PlayersBoxes/SB_102_6H.SB_102_6H")
        (Components|Activation|Activate _signaljammer_h false)
        (Audio|Components|Audio|SetSound _signaljammer_c "/Game/AdvancedVoIPVoiceChatSystem/Audio/Radio_Buses/PlayersBoxes/SB_102_6C.SB_102_6C")
        (Components|Activation|Activate _signaljammer_c false)
        (Development|PrintString "102"))
      (:NewEnumerator2
        (Audio|Components|Audio|SetSound _audio "/Game/AdvancedVoIPVoiceChatSystem/Audio/Radio_Buses/SB_radioSourceBus_104_0.SB_radioSourceBus_104_0")
        (Components|Activation|Activate _audio false)
        (Audio|Components|Audio|SetSound _signaljammer_l "/Game/AdvancedVoIPVoiceChatSystem/Audio/Radio_Buses/PlayersBoxes/SB_104_0L.SB_104_0L")
        (Components|Activation|Activate _signaljammer_l false)
        (Audio|Components|Audio|SetSound _signaljammer_m "/Game/AdvancedVoIPVoiceChatSystem/Audio/Radio_Buses/PlayersBoxes/SB_104_0M.SB_104_0M")
        (Components|Activation|Activate _signaljammer_m false)
        (Audio|Components|Audio|SetSound _signaljammer_m1 "/Game/AdvancedVoIPVoiceChatSystem/Audio/Radio_Buses/PlayersBoxes/SB_104_0M1.SB_104_0M1")
        (Components|Activation|Activate _signaljammer_m1 false)
        (Audio|Components|Audio|SetSound _signaljammer_h "/Game/AdvancedVoIPVoiceChatSystem/Audio/Radio_Buses/PlayersBoxes/SB_104_0H.SB_104_0H")
        (Components|Activation|Activate _signaljammer_h false)
        (Audio|Components|Audio|SetSound _signaljammer_c "/Game/AdvancedVoIPVoiceChatSystem/Audio/Radio_Buses/PlayersBoxes/SB_104_0C.SB_104_0C")
        (Components|Activation|Activate _signaljammer_c false)
        (Development|PrintString "104")))
    (else
      (Components|Activation|Deactivate (Variables|Default|GetAudio))
      (Components|Activation|Deactivate _signaljammer_l)
      (Components|Activation|Deactivate _signaljammer_m)
      (Components|Activation|Deactivate _signaljammer_m1)
      (Components|Activation|Deactivate _signaljammer_h)
      (Components|Activation|Deactivate _signaljammer_c)
      (Components|Activation|Deactivate (Variables|Default|GetBeepBusOnly))
      (Components|Activation|Deactivate (Variables|Default|GetBeepSelfReply))
      (Components|Activation|Deactivate (Variables|Default|GetStaticSoundBusOnly)))))

(event EventActivateReceiverOutput
  (bind _signaljammer_m (Variables|Default|GetSignalJammer_M))
  (bind _signaljammer_l (Variables|Default|GetSignalJammer_L))
  (bind _signaljammer_m1 (Variables|Default|GetSignalJammer_M1))
  (bind _signaljammer_h (Variables|Default|GetSignalJammer_H))
  (bind _signaljammer_c (Variables|Default|GetSignalJammer_C))
  (bind _audio (Variables|Default|GetAudio))
  (if (Variables|Default|GetisWalkieTalkieOn?)
    (switch Utilities|FlowControl|Switch|SwitchonE_RadioFrequencies (Variables|Default|GetFrequencies)
      (:NewEnumerator0
        (Audio|Components|Audio|SetSound _audio "/Game/AdvancedVoIPVoiceChatSystem/Audio/Radio_Buses/SB_radioSourceBus_99_1.SB_radioSourceBus_99_1")
        (Components|Activation|Activate _audio false)
        (Audio|Components|Audio|SetSound _signaljammer_l "/Game/AdvancedVoIPVoiceChatSystem/Audio/Radio_Buses/PlayersBoxes/SB_99_1L.SB_99_1L")
        (Components|Activation|Activate _signaljammer_l false)
        (Audio|Components|Audio|SetSound _signaljammer_m "/Game/AdvancedVoIPVoiceChatSystem/Audio/Radio_Buses/PlayersBoxes/SB_99_1M.SB_99_1M")
        (Components|Activation|Activate _signaljammer_m false)
        (Audio|Components|Audio|SetSound _signaljammer_m1 "/Game/AdvancedVoIPVoiceChatSystem/Audio/Radio_Buses/PlayersBoxes/SB_99_1M1.SB_99_1M1")
        (Components|Activation|Activate _signaljammer_m1 false)
        (Audio|Components|Audio|SetSound _signaljammer_h "/Game/AdvancedVoIPVoiceChatSystem/Audio/Radio_Buses/PlayersBoxes/SB_99_1H.SB_99_1H")
        (Components|Activation|Activate _signaljammer_h false)
        (Audio|Components|Audio|SetSound _signaljammer_c "/Game/AdvancedVoIPVoiceChatSystem/Audio/Radio_Buses/PlayersBoxes/SB_99_1C.SB_99_1C")
        (Components|Activation|Activate _signaljammer_c false)
        (Development|PrintString "99"))
      (:NewEnumerator1
        (Audio|Components|Audio|SetSound _audio "/Game/AdvancedVoIPVoiceChatSystem/Audio/Radio_Buses/SB_radioSourceBus_102_6.SB_radioSourceBus_102_6")
        (Components|Activation|Activate _audio false)
        (Audio|Components|Audio|SetSound _signaljammer_l "/Game/AdvancedVoIPVoiceChatSystem/Audio/Radio_Buses/PlayersBoxes/SB_102_6L.SB_102_6L")
        (Components|Activation|Activate _signaljammer_l false)
        (Audio|Components|Audio|SetSound _signaljammer_m "/Game/AdvancedVoIPVoiceChatSystem/Audio/Radio_Buses/PlayersBoxes/SB_102_6M.SB_102_6M")
        (Components|Activation|Activate _signaljammer_m false)
        (Audio|Components|Audio|SetSound _signaljammer_m1 "/Game/AdvancedVoIPVoiceChatSystem/Audio/Radio_Buses/PlayersBoxes/SB_102_6M1.SB_102_6M1")
        (Components|Activation|Activate _signaljammer_m1 false)
        (Audio|Components|Audio|SetSound _signaljammer_h "/Game/AdvancedVoIPVoiceChatSystem/Audio/Radio_Buses/PlayersBoxes/SB_102_6H.SB_102_6H")
        (Components|Activation|Activate _signaljammer_h false)
        (Audio|Components|Audio|SetSound _signaljammer_c "/Game/AdvancedVoIPVoiceChatSystem/Audio/Radio_Buses/PlayersBoxes/SB_102_6C.SB_102_6C")
        (Components|Activation|Activate _signaljammer_c false)
        (Development|PrintString "102"))
      (:NewEnumerator2
        (Audio|Components|Audio|SetSound _audio "/Game/AdvancedVoIPVoiceChatSystem/Audio/Radio_Buses/SB_radioSourceBus_104_0.SB_radioSourceBus_104_0")
        (Components|Activation|Activate _audio false)
        (Audio|Components|Audio|SetSound _signaljammer_l "/Game/AdvancedVoIPVoiceChatSystem/Audio/Radio_Buses/PlayersBoxes/SB_104_0L.SB_104_0L")
        (Components|Activation|Activate _signaljammer_l false)
        (Audio|Components|Audio|SetSound _signaljammer_m "/Game/AdvancedVoIPVoiceChatSystem/Audio/Radio_Buses/PlayersBoxes/SB_104_0M.SB_104_0M")
        (Components|Activation|Activate _signaljammer_m false)
        (Audio|Components|Audio|SetSound _signaljammer_m1 "/Game/AdvancedVoIPVoiceChatSystem/Audio/Radio_Buses/PlayersBoxes/SB_104_0M1.SB_104_0M1")
        (Components|Activation|Activate _signaljammer_m1 false)
        (Audio|Components|Audio|SetSound _signaljammer_h "/Game/AdvancedVoIPVoiceChatSystem/Audio/Radio_Buses/PlayersBoxes/SB_104_0H.SB_104_0H")
        (Components|Activation|Activate _signaljammer_h false)
        (Audio|Components|Audio|SetSound _signaljammer_c "/Game/AdvancedVoIPVoiceChatSystem/Audio/Radio_Buses/PlayersBoxes/SB_104_0C.SB_104_0C")
        (Components|Activation|Activate _signaljammer_c false)
        (Development|PrintString "104")))
    (else
      (Components|Activation|Deactivate (Variables|Default|GetAudio))
      (Components|Activation|Deactivate _signaljammer_l)
      (Components|Activation|Deactivate _signaljammer_m)
      (Components|Activation|Deactivate _signaljammer_m1)
      (Components|Activation|Deactivate _signaljammer_h)
      (Components|Activation|Deactivate _signaljammer_c)
      (Components|Activation|Deactivate (Variables|Default|GetBeepBusOnly))
      (Components|Activation|Deactivate (Variables|Default|GetBeepSelfReply))
      (Components|Activation|Deactivate (Variables|Default|GetStaticSoundBusOnly)))))

(fn ConstructionScript
  (|CallParentFunction))

(fn OnRepFrequencies)

(fn BPIWalkieTalkieSingleBandRef
  (return self))

(fn BPIWalkieTalkieMultiBandRef
  (return self))