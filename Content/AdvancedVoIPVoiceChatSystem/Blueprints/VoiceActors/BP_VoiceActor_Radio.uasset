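; Radio voice actor for the voice chat system, providing a singleplayer path that uses Audio Capture because VoIP needs a session.
; Start and stop events activate or deactivate a passed-in Audio Capture component together with the actor's Audio component.
; Comments describe routing the captured voice through a submix or source bus effect; an unwired test node would activate OutputAudioCapture.
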(event Custom|SentSubmitToRadio
  (params (AudioCaptureComponent :type Audio%20Capture%20Component%20Object%20Reference))
  ;[1 1 1] For SinglePlayer here
  ;;[0 0 0] When you are playing Singleplayer "sent source bus post effect node OR sent to submix node your voice with Audio Capture Component instead because you cannot use VoIP without a session
  (Components|Activation|Activate AudioCaptureComponent false)
  (Components|Activation|Activate (Variables|Default|GetAudio) false))

(event Custom|StopSubmitToRadio
  (params (AudioCaptureComponent :type Audio%20Capture%20Component%20Object%20Reference))
  ;[1 1 1] For SinglePlayer here
  (Components|Activation|Deactivate AudioCaptureComponent)
  (Components|Activation|Deactivate (Variables|Default|GetAudio)))

(fn ConstructionScript
  (|CallParentFunction))