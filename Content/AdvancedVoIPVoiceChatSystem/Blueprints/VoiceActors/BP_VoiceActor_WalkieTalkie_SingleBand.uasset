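; Single-band walkie-talkie voice actor for multiplayer voice chat, with replicated power and transmit states.
; Server events set those states and relay screen and speaking material color and emission changes via multicasts.
; A power dispatcher, bound by multicast on BeginPlay, toggles receiver audio and signal-jammer components through cross-resetting DoOnce gates, also silencing beep and static on power-off.
; Destruction disables the HUD's frequency text, and an interface returns this actor.
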(event Custom|Mcast_ActivateScreenEmission
  (Rendering|Material|SetVectorParameterValueonMaterials (Variables|Default|GetVoiceActor) "Color" "0,1.000000, 0")
  (Rendering|Material|SetScalarParameterValueonMaterials (Variables|Default|GetVoiceActor) "Emission" 2e+01))

(event Custom|Mcast_DeactivateScreenEmission
  (Rendering|Material|SetVectorParameterValueonMaterials (Variables|Default|GetVoiceActor) "Color" "1.000000,0.000000, 0")
  (Rendering|Material|SetScalarParameterValueonMaterials (Variables|Default|GetVoiceActor) "Emission" 2e+01))

(event Custom|DeactivateReceiverOutput
  (bind _signaljammer_m (Variables|Default|GetSignalJammer_M))
  (bind _signaljammer_l (Variables|Default|GetSignalJammer_L))
  (bind _signaljammer_m1 (Variables|Default|GetSignalJammer_M1))
  (bind _signaljammer_h (Variables|Default|GetSignalJammer_H))
  (bind _signaljammer_c (Variables|Default|GetSignalJammer_C))
  (bind _audio (Variables|Default|GetAudio))
  ;[1 0 0] You must use SignalJammer Seperate SoundBus BUT because it is 1 frequency for the time being keep it at 99.1 for example because in the end of the day singleBand is still 1 frequency!
  (if (Variables|Default|GetisWalkieTalkieOn?)
    (Utilities|FlowControl|DoOnce false :!label _label
      (:Completed
        (Components|Activation|Activate _audio false)
        (Components|Activation|Activate _signaljammer_l false)
        (Components|Activation|Activate _signaljammer_m false)
        (Components|Activation|Activate _signaljammer_m1 false)
        (Components|Activation|Activate _signaljammer_h false)
        (Components|Activation|Activate _signaljammer_c false)
        (goto _label_2 Reset)))
    (else
      (Utilities|FlowControl|DoOnce false :!label _label_2
        (:Completed
          (Components|Activation|Deactivate _audio)
          (Components|Activation|Deactivate _signaljammer_l)
          (Components|Activation|Deactivate _signaljammer_m)
          (Components|Activation|Deactivate _signaljammer_m1)
          (Components|Activation|Deactivate _signaljammer_h)
          (Components|Activation|Deactivate _signaljammer_c)
          (Components|Activation|Deactivate (Variables|Default|GetBeepBusOnly))
          (Components|Activation|Deactivate (Variables|Default|GetBeepSelfReply))
          (Components|Activation|Deactivate (Variables|Default|GetStaticSoundBusOnly))
          (goto _label Reset))))))

(event Custom|SRV_isWalkieTalkieON?
  (params (isWalkieTalkieOn? :type Boolean))
  (Variables|Default|SetisWalkieTalkieOn? isWalkieTalkieOn?))

(event Custom|SRV_isWalkieTalkieTransmiting?
  (params (isWalkieTalkieTransmiting? :type Boolean))
  (Variables|Default|SetisWalkieTalkieTransmiting? isWalkieTalkieTransmiting?))

(event Custom|isWalkieTalkieOn?_Dispatcher_Event
  (if (Variables|Default|GetisWalkieTalkieOn?)
    (CallFunction|ActivateReceiverOutput)
    (else
      (CallFunction|DeactivateReceiverOutput))))

(event Custom|SRV_ListenON?
  (CallFunction|MCastListenON?))

(event Custom|MCast_ListenON?
  ;[1 1 1 1 12] Remove Reliable? (works but if it double acts then remove it?)
  (EventDispatchers|BindEventtoIsWalkieTalkieOn?Dispatcher (delegate Custom|isWalkieTalkieOn?_Dispatcher_Event)))

(event Custom|SRV_ActivateScreenEmission
  (CallFunction|McastActivateScreenEmission))

(event Custom|SRV_DeactivateScreenEmission
  (CallFunction|McastDeactivateScreenEmission))

(event Custom|SRV_SetTransmitingON_S
  (Variables|Default|SetisWalkieTalkieTransmiting? true))

(event Custom|SRV_SetTransmittingOFF_S
  (Variables|Default|SetisWalkieTalkieTransmiting? false))

(event Custom|SRV_wtON_S
  (Variables|Default|SetisWalkieTalkieOn? true)
  (Default|CallIsWalkieTalkieOn?Dispatcher))

(event Custom|SRV_wtOFF_S
  (Variables|Default|SetisWalkieTalkieOn? false)
  (Default|CallIsWalkieTalkieOn?Dispatcher))

(event Custom|SRV_ActivateSpeakingEmission
  (CallFunction|McastActivateSpeakingEmission))

(event Custom|SRV_DeactivateSpeakingEmission
  (CallFunction|McastDeactivateSpeakingEmission))

(event Custom|Mcast_ActivateSpeakingEmission
  (Rendering|Material|SetVectorParameterValueonMaterials (Variables|Default|GetVoiceActor) "Color" "1.000000,0.000000,0.000000")
  (Rendering|Material|SetScalarParameterValueonMaterials (Variables|Default|GetVoiceActor) "Emission" 2e+01))

(event Custom|Mcast_DeactivateSpeakingEmission
  (Rendering|Material|SetVectorParameterValueonMaterials (Variables|Default|GetVoiceActor) "Color" "1.000000,0.000000,0.000000")
  (Rendering|Material|SetScalarParameterValueonMaterials (Variables|Default|GetVoiceActor) "Emission" 0.0))

(event Custom|ActivateReceiverOutput
  (bind _signaljammer_m (Variables|Default|GetSignalJammer_M))
  (bind _signaljammer_l (Variables|Default|GetSignalJammer_L))
  (bind _signaljammer_m1 (Variables|Default|GetSignalJammer_M1))
  (bind _signaljammer_h (Variables|Default|GetSignalJammer_H))
  (bind _signaljammer_c (Variables|Default|GetSignalJammer_C))
  (bind _audio (Variables|Default|GetAudio))
  ;[1 0 0] You must use SignalJammer Seperate SoundBus BUT because it is 1 frequency for the time being keep it at 99.1 for example because in the end of the day singleBand is still 1 frequency!
  (if (Variables|Default|GetisWalkieTalkieOn?)
    (Utilities|FlowControl|DoOnce false :!label _label
      (:Completed
        (Components|Activation|Activate _audio false)
        (Components|Activation|Activate _signaljammer_l false)
        (Components|Activation|Activate _signaljammer_m false)
        (Components|Activation|Activate _signaljammer_m1 false)
        (Components|Activation|Activate _signaljammer_h false)
        (Components|Activation|Activate _signaljammer_c false)
        (goto _label_2 Reset)))
    (else
      (Utilities|FlowControl|DoOnce false :!label _label_2
        (:Completed
          (Components|Activation|Deactivate _audio)
          (Components|Activation|Deactivate _signaljammer_l)
          (Components|Activation|Deactivate _signaljammer_m)
          (Components|Activation|Deactivate _signaljammer_m1)
          (Components|Activation|Deactivate _signaljammer_h)
          (Components|Activation|Deactivate _signaljammer_c)
          (Components|Activation|Deactivate (Variables|Default|GetBeepBusOnly))
          (Components|Activation|Deactivate (Variables|Default|GetBeepSelfReply))
          (Components|Activation|Deactivate (Variables|Default|GetStaticSoundBusOnly))
          (goto _label Reset))))))

(event EventBeginPlay
  (|CallParentFunction)
  (CallFunction|SRVListenON?))

(event EventDestroyed
  (bind _returnvalue (Game|GetInstigatorController))
  (Utilities|IsValid _returnvalue
    (:Is%20Valid
      (bind _characterref (Class|BPIVoiceChatCharacter|BPIVoiceChatCharacterPlayerMPRef(Message) (Pawn|GetControlledPawn _returnvalue)))
      (Utilities|IsValid (Variables|/Game/AdvancedVoIPVoiceChatSystem/Blueprints/CharacterBP/Multiplayer/BP_VoiceChat_Character_White.BP_VoiceChat_Character_White_C|GetHudRef _characterref)
        (:Is%20Valid
          (Default|TextFrequencyChangeDisable (Variables|/Game/AdvancedVoIPVoiceChatSystem/Widgets/WB_Player_HUD.WB_Player_HUD_C|GetWB_UI_WT (Variables|/Game/AdvancedVoIPVoiceChatSystem/Blueprints/CharacterBP/Multiplayer/BP_VoiceChat_Character_White.BP_VoiceChat_Character_White_C|GetHudRef _characterref))))))))

(fn ConstructionScript
  (|CallParentFunction)
  (bind _returnvalue (Rendering|Material|CreateDynamicMaterialInstance (Variables|Default|GetVoiceActor) 1 "/Game/AdvancedVoIPVoiceChatSystem/Materials/MI_Radio_Mobile_Screen_Inst.MI_Radio_Mobile_Screen_Inst" "None" :!class /Script/Engine.PrimitiveComponent))
  (Variables|Default|SetScreenColorEmission _returnvalue)
  (Rendering|Material|SetMaterial (Variables|Default|GetVoiceActor) 1 (Variables|Default|GetScreenColorEmission)))

(fn OnRepIsWalkieTalkieOn?
  (bind _audio (Variables|Default|GetAudio))
  (if (Variables|Default|GetisWalkieTalkieOn?)
    (Utilities|FlowControl|DoOnce false :!label _label
      (:Completed
        (Components|Activation|Activate _audio false)
        (goto _label_2 Reset)))
    (else
      (Utilities|FlowControl|DoOnce false :!label _label_2
        (:Completed
          (Components|Activation|Deactivate _audio)
          (goto _label Reset))))))

(fn OnRepIsWalkieTalkieTransmiting?)

(fn BPIWalkieTalkieMultiBandRef
  (return 0))

(fn BPIWalkieTalkieSingleBandRef
  (return self))