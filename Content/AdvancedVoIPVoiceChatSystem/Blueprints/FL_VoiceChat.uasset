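; Voice chat function library that resolves players for the VoIP system by circuit number or name.
; GetMapPlayerDatabase reads the player-to-circuit map through a game mode interface, using the key at the given position to index the values and return that controller's pawn.
; RequestRemotePlayerNumber searches the GameState PlayerArray for a matching player name and returns its array index.
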(fn GetMapPlayerDatabase
  (params (CircuitNumber :type Integer))
  (bind _gamemodemultiplayer (Class|BPIGMVoiceChat|BPIGMVoiceChatRef(Message) (Game|GetGameMode)))
  (bind _keys (Utilities|Map|Keys (Variables|/Game/AdvancedVoIPVoiceChatSystem/Blueprints/Modes/BP_GM_VoiceChat_MP.BP_GM_VoiceChat_MP_C|GetPlayerAndCircuitNumberBurnedIn _gamemodemultiplayer)))
  (bind _values (Utilities|Map|Values (Variables|/Game/AdvancedVoIPVoiceChatSystem/Blueprints/Modes/BP_GM_VoiceChat_MP.BP_GM_VoiceChat_MP_C|GetPlayerAndCircuitNumberBurnedIn _gamemodemultiplayer)))
  (return (Pawn|GetControlledPawn (Utilities|Array|Get(acopy) _values (Utilities|Array|Get(acopy) _keys CircuitNumber)))))

(fn RequestRemotePlayerNumber
  (params (PlayerName :type Text))
  (for (_array_element _array_index) (Variables|/Script/Engine.GameStateBase|GetPlayerArray (Game|GetGameState))
    (if (Utilities|Enum|Equal(Enum) (PlayerState|GetPlayerName _array_element) (Utilities|String|ToString(Text) PlayerName))
      (return _array_index))))