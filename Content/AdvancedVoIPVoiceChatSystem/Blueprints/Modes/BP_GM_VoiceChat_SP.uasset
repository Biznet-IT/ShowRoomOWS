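; BP_GM_VoiceChat_SP is the single-player Game Mode of the voice chat system, marked as deletable showcase code.
; On BeginPlay it turns off OSS voice loopback, then applies lowest-quality, windowed, frame-capped GameUserSettings for testing on low settings.
; Unconnected console-command nodes remain as an alternative way to lower the graphics settings.
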(event EventBeginPlay
  ;[0 0 0 1 24] #ShowCaseCode #deleteItIfYouWant no depencies here .. BP_GM_VoiceChat_SP SP stands for SinglePlayer
  ;;[1 1 1] Low Quality Settings Connect/Disconnect this to Begin Play if you want to test with lowest settings enabled on the hosts
  (Development|ExecuteConsoleCommand "OSS.VoiceLoopback 0" 0)
  (bind _returnvalue (Settings|GetGameUserSettings))
  (Class|GameUserSettings|SetScreenResolution _returnvalue (Variables|Default|GetScreenRes))
  (Class|GameUserSettings|SetViewDistanceQuality _returnvalue)
  (Class|GameUserSettings|SetPostProcessingQuality _returnvalue)
  (Class|GameUserSettings|SetShadowQuality _returnvalue)
  (Class|GameUserSettings|SetTextureQuality _returnvalue)
  (Class|GameUserSettings|SetResolutionScaleValueEx _returnvalue 0.0)
  (Class|GameUserSettings|SetFrameRateLimit _returnvalue 3e+01)
  (Class|GameUserSettings|SetFullscreenMode _returnvalue "Windowed")
  (Class|GameUserSettings|ApplySettings _returnvalue false))

(fn ConstructionScript)