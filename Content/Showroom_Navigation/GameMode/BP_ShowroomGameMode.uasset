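; Showroom game mode that exercises inherited calls for world time, zones and global data, reporting results as debug prints.
; On BeginPlay it requests the current world time, and notify and error events print the result.
; Other notify handlers print zone additions, global data keys and running zone instances with port and status.
; Sample calls to add a zone and to write or read global data are left unconnected.
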(event Custom|Event%20Notify%20Add%20Zone
  (Development|PrintString "Zone Added!"))

(event Custom|Event%20Notify%20Get%20Current%20World%20Time
  (params (CurrentWorldTime :type Float%20%28single-precision%29))
  (Development|PrintString (Utilities|String|Append "Current Game World Time: " (Utilities|String|ToString(Float) CurrentWorldTime))))

(event Custom|Event%20Error%20Get%20Current%20World%20Time
  (params (ErrorMsg :type String))
  (Development|PrintString ErrorMsg))

(event Custom|Event%20Notify%20Get%20Global%20Data%20Item
  (params (GlobalDataKey :type String))
  (Development|PrintString (Utilities|String|Append "Global Data Item: " GlobalDataKey)))

(event Custom|Event%20Notify%20Add%20or%20Update%20Global%20Data%20Item)

(event Custom|Event%20Notify%20Get%20Zone%20Instances%20for%20Zone
  (params (ZoneInstances :type Array%20of%20Zone%20Instance%20Structures))
  (Development|PrintString "List of running Game Instances:")
  (for _array_element ZoneInstances
    (Development|PrintString (Utilities|String|Append (.ZoneName (Utilities|Struct|BreakZoneInstance _array_element)) " - Port: " (Utilities|String|ToString(Integer) (.Port (Utilities|Struct|BreakZoneInstance _array_element))) " - Status: " (Utilities|String|ToString(Integer) (.Status (Utilities|Struct|BreakZoneInstance _array_element)))))))

(event EventBeginPlay
  (Class|OWSGameMode|GetCurrentWorldTime))

(fn ConstructionScript)