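; Game state Blueprint for the showroom's complex detail view, switching the player into focus-point navigation on BeginPlay.
; It clears all widgets, checks for the showroom game instance, possesses the level's BP_FocusPawnComplex and adds the WBP_FocusPoint_complex UI to the viewport.
; FPShowHideTagObjectsFunction is empty; its disconnected logic would hide level and waypoint actors and show focus-point actors from game instance arrays.
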(event EventBeginPlay
  (bind _returnvalue (Game|GetPlayerController 0))
  ;[1 1 1] Posses Simple Pawn and Menue
  (Viewport|RemoveAllWidgets)
  (Utilities|Casting|CastToBP_Gameinstance_showroom (Game|GetGameInstance))
  (bind _returnvalue_2 (Actor|GetActorOfClass "/Game/Showroom_Navigation/Blueprint/FocusPoint_Complex/BP_FocusPawnComplex.BP_FocusPawnComplex_C"))
  (Pawn|Possess _returnvalue _returnvalue_2)
  (bind _returnvalue_3 (UserInterface|CreateWidget "/Game/Showroom_Navigation/Blueprint/UI_Widget/WBP_FocusPoint_complex.WBP_FocusPoint_complex_C" _returnvalue))
  (UserInterface|Viewport|AddtoViewport _returnvalue_3 0))

(fn ConstructionScript)

(fn FPShow/HideTagObjectsFunction)