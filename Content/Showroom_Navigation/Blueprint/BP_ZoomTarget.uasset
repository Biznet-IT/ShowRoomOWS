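; Showroom zoom-point actor that serves as a clickable hotspot for camera focus, shown as either a billboard with optional camera-facing label or a 3D button.
; The construction script sets up its preview spring-arm camera, icon and optional pano marker.
; Click or non-drag touch writes its focus index, arm length and tour index to BP_Gameinstance_showroom, then fires the RunFocus dispatcher.
; TourButtonLabels supplies a custom or display-name-derived tour name.
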(event OnClicked(Box_Trigger)
  (params (TouchedComponent :type Primitive%20Component%20Object%20Reference) (ButtonPressed :type Key%20Structure))
  (bind _self self)
  ;[1 1 1] Do not click when Touch is moving
  (bind _asbp_gameinstance_showroom (Utilities|Casting|CastToBP_Gameinstance_showroom (Game|GetGameInstance)))
  (if (not (Variables|/Game/Showroom_Navigation/Gameinstance/BP_Gameinstance_showroom.BP_Gameinstance_showroom_C|Getis%20first%20touch _asbp_gameinstance_showroom))
    ;[1 1 1] Find_this ZoomPoint in Array
    (bind _asbp_gameinstance_showroom_2 (Utilities|Casting|CastToBP_Gameinstance_showroom (Game|GetGameInstance)))
    (Variables|/Game/Showroom_Navigation/Gameinstance/BP_Gameinstance_showroom.BP_Gameinstance_showroom_C|SetGI_GetFocus _asbp_gameinstance_showroom_2 (Utilities|Array|FindItem (Variables|/Game/Showroom_Navigation/Gameinstance/BP_Gameinstance_showroom.BP_Gameinstance_showroom_C|GetZoomPoint_Array _asbp_gameinstance_showroom_2) self))
    ;[1 1 1] Fire dispatcher to Pawn
    (Variables|/Game/Showroom_Navigation/Gameinstance/BP_Gameinstance_showroom.BP_Gameinstance_showroom_C|SetGI_ArmLength_LevelSwitch _asbp_gameinstance_showroom_2 (Variables|Default|GetZoomInPoint01Armlength))
    (bind _asbp_gameinstance_showroom_3 (Utilities|Casting|CastToBP_Gameinstance_showroom (Game|GetGameInstance)))
    (if (Utilities|Array|ContainsItem (Variables|/Game/Showroom_Navigation/Gameinstance/BP_Gameinstance_showroom.BP_Gameinstance_showroom_C|GetGI_TourArray _asbp_gameinstance_showroom_3) _self)
      (Variables|/Game/Showroom_Navigation/Gameinstance/BP_Gameinstance_showroom.BP_Gameinstance_showroom_C|SetGI_Tour_Button_index _asbp_gameinstance_showroom_3 (Utilities|Array|FindItem (Variables|/Game/Showroom_Navigation/Gameinstance/BP_Gameinstance_showroom.BP_Gameinstance_showroom_C|GetGI_TourArray _asbp_gameinstance_showroom_3) _self))
      (else
        (Variables|/Game/Showroom_Navigation/Gameinstance/BP_Gameinstance_showroom.BP_Gameinstance_showroom_C|SetGI_Tour_Button_index _asbp_gameinstance_showroom_3 -500)))
    (Default|CallEventDispatcherRunFocus)))

(event OnInputTouchEnd(Click_Highlight)
  (params (FingerIndex :type ETouchIndex%20Enum :default "Touch1") (TouchedComponent :type Primitive%20Component%20Object%20Reference))
  (bind _self self)
  ;[1 1 1] Do not click when Touc is moving
  (bind _asbp_gameinstance_showroom (Utilities|Casting|CastToBP_Gameinstance_showroom (Game|GetGameInstance)))
  (if (not (Variables|/Game/Showroom_Navigation/Gameinstance/BP_Gameinstance_showroom.BP_Gameinstance_showroom_C|Getis_Touch_moving _asbp_gameinstance_showroom))
    ;[1 1 1] Find_this ZoomPoint in Array
    (bind _asbp_gameinstance_showroom_2 (Utilities|Casting|CastToBP_Gameinstance_showroom (Game|GetGameInstance)))
    (Variables|/Game/Showroom_Navigation/Gameinstance/BP_Gameinstance_showroom.BP_Gameinstance_showroom_C|SetGI_GetFocus _asbp_gameinstance_showroom_2 (Utilities|Array|FindItem (Variables|/Game/Showroom_Navigation/Gameinstance/BP_Gameinstance_showroom.BP_Gameinstance_showroom_C|GetZoomPoint_Array _asbp_gameinstance_showroom_2) self))
    ;[1 1 1] Fire dispatcher to Pawn
    (Variables|/Game/Showroom_Navigation/Gameinstance/BP_Gameinstance_showroom.BP_Gameinstance_showroom_C|SetGI_ArmLength_LevelSwitch _asbp_gameinstance_showroom_2 (Variables|Default|GetZoomInPoint01Armlength))
    (bind _asbp_gameinstance_showroom_3 (Utilities|Casting|CastToBP_Gameinstance_showroom (Game|GetGameInstance)))
    (if (Utilities|Array|ContainsItem (Variables|/Game/Showroom_Navigation/Gameinstance/BP_Gameinstance_showroom.BP_Gameinstance_showroom_C|GetGI_TourArray _asbp_gameinstance_showroom_3) _self)
      (Variables|/Game/Showroom_Navigation/Gameinstance/BP_Gameinstance_showroom.BP_Gameinstance_showroom_C|SetGI_Tour_Button_index _asbp_gameinstance_showroom_3 (Utilities|Array|FindItem (Variables|/Game/Showroom_Navigation/Gameinstance/BP_Gameinstance_showroom.BP_Gameinstance_showroom_C|GetGI_TourArray _asbp_gameinstance_showroom_3) _self))
      (else
        (Variables|/Game/Showroom_Navigation/Gameinstance/BP_Gameinstance_showroom.BP_Gameinstance_showroom_C|SetGI_Tour_Button_index _asbp_gameinstance_showroom_3 -500)))
    (Default|CallEventDispatcherRunFocus)))

(event OnInputTouchEnd(Box_Trigger)
  (params (FingerIndex :type ETouchIndex%20Enum :default "Touch1") (TouchedComponent :type Primitive%20Component%20Object%20Reference))
  (bind _self self)
  ;[1 1 1] Do not click when Touch is moving
  (bind _asbp_gameinstance_showroom (Utilities|Casting|CastToBP_Gameinstance_showroom (Game|GetGameInstance)))
  (if (not (Variables|/Game/Showroom_Navigation/Gameinstance/BP_Gameinstance_showroom.BP_Gameinstance_showroom_C|Getis_Touch_moving _asbp_gameinstance_showroom))
    ;[1 1 1] Find_this ZoomPoint in Array
    (bind _asbp_gameinstance_showroom_2 (Utilities|Casting|CastToBP_Gameinstance_showroom (Game|GetGameInstance)))
    (Variables|/Game/Showroom_Navigation/Gameinstance/BP_Gameinstance_showroom.BP_Gameinstance_showroom_C|SetGI_GetFocus _asbp_gameinstance_showroom_2 (Utilities|Array|FindItem (Variables|/Game/Showroom_Navigation/Gameinstance/BP_Gameinstance_showroom.BP_Gameinstance_showroom_C|GetZoomPoint_Array _asbp_gameinstance_showroom_2) self))
    ;[1 1 1] Fire dispatcher to Pawn
    (Variables|/Game/Showroom_Navigation/Gameinstance/BP_Gameinstance_showroom.BP_Gameinstance_showroom_C|SetGI_ArmLength_LevelSwitch _asbp_gameinstance_showroom_2 (Variables|Default|GetZoomInPoint01Armlength))
    (bind _asbp_gameinstance_showroom_3 (Utilities|Casting|CastToBP_Gameinstance_showroom (Game|GetGameInstance)))
    (if (Utilities|Array|ContainsItem (Variables|/Game/Showroom_Navigation/Gameinstance/BP_Gameinstance_showroom.BP_Gameinstance_showroom_C|GetGI_TourArray _asbp_gameinstance_showroom_3) _self)
      (Variables|/Game/Showroom_Navigation/Gameinstance/BP_Gameinstance_showroom.BP_Gameinstance_showroom_C|SetGI_Tour_Button_index _asbp_gameinstance_showroom_3 (Utilities|Array|FindItem (Variables|/Game/Showroom_Navigation/Gameinstance/BP_Gameinstance_showroom.BP_Gameinstance_showroom_C|GetGI_TourArray _asbp_gameinstance_showroom_3) _self))
      (else
        (Variables|/Game/Showroom_Navigation/Gameinstance/BP_Gameinstance_showroom.BP_Gameinstance_showroom_C|SetGI_Tour_Button_index _asbp_gameinstance_showroom_3 -500)))
    (Default|CallEventDispatcherRunFocus)))

(event OnClicked(Click_Highlight)
  (params (TouchedComponent :type Primitive%20Component%20Object%20Reference) (ButtonPressed :type Key%20Structure))
  (bind _self self)
  ;[1 1 1] Do not click when Touc is moving
  (bind _asbp_gameinstance_showroom (Utilities|Casting|CastToBP_Gameinstance_showroom (Game|GetGameInstance)))
  (if (not (Variables|/Game/Showroom_Navigation/Gameinstance/BP_Gameinstance_showroom.BP_Gameinstance_showroom_C|Getis%20first%20touch _asbp_gameinstance_showroom))
    ;[1 1 1] Find_this ZoomPoint in Array
    (bind _asbp_gameinstance_showroom_2 (Utilities|Casting|CastToBP_Gameinstance_showroom (Game|GetGameInstance)))
    (Variables|/Game/Showroom_Navigation/Gameinstance/BP_Gameinstance_showroom.BP_Gameinstance_showroom_C|SetGI_GetFocus _asbp_gameinstance_showroom_2 (Utilities|Array|FindItem (Variables|/Game/Showroom_Navigation/Gameinstance/BP_Gameinstance_showroom.BP_Gameinstance_showroom_C|GetZoomPoint_Array _asbp_gameinstance_showroom_2) self))
    ;[1 1 1] Fire dispatcher to Pawn
    (Variables|/Game/Showroom_Navigation/Gameinstance/BP_Gameinstance_showroom.BP_Gameinstance_showroom_C|SetGI_ArmLength_LevelSwitch _asbp_gameinstance_showroom_2 (Variables|Default|GetZoomInPoint01Armlength))
    (bind _asbp_gameinstance_showroom_3 (Utilities|Casting|CastToBP_Gameinstance_showroom (Game|GetGameInstance)))
    (if (Utilities|Array|ContainsItem (Variables|/Game/Showroom_Navigation/Gameinstance/BP_Gameinstance_showroom.BP_Gameinstance_showroom_C|GetGI_TourArray _asbp_gameinstance_showroom_3) _self)
      (Variables|/Game/Showroom_Navigation/Gameinstance/BP_Gameinstance_showroom.BP_Gameinstance_showroom_C|SetGI_Tour_Button_index _asbp_gameinstance_showroom_3 (Utilities|Array|FindItem (Variables|/Game/Showroom_Navigation/Gameinstance/BP_Gameinstance_showroom.BP_Gameinstance_showroom_C|GetGI_TourArray _asbp_gameinstance_showroom_3) _self))
      (else
        (Variables|/Game/Showroom_Navigation/Gameinstance/BP_Gameinstance_showroom.BP_Gameinstance_showroom_C|SetGI_Tour_Button_index _asbp_gameinstance_showroom_3 -500)))
    (Default|CallEventDispatcherRunFocus)))

(event OnBeginCursorOver(Click_Highlight)
  (params (TouchedComponent :type Primitive%20Component%20Object%20Reference))
  ;[1 1 1] ClickHighlight Mouseover
  (Rendering|SetVisibility (Variables|Default|GetClick_Highlight) true false))

(event OnEndCursorOver(Click_Highlight)
  (params (TouchedComponent :type Primitive%20Component%20Object%20Reference))
  ;[1 1 1] ClickHighlight Mouseover
  (Rendering|SetVisibility (Variables|Default|GetClick_Highlight) false false))

(event EventBeginPlay
  (bind _icondummy_transform (Variables|Default|GetIconDummy_transform))
  (bind _defaultsceneroot (Variables|Default|GetDefaultSceneRoot))
  (bind _icondummy_transform_2 (Variables|Default|GetIconDummy_transform))
  (bind _returnvalue (Transformation|GetRelativeTransform _icondummy_transform))
  (bind _relativelocation (Variables|/Script/Engine.SceneComponent|GetRelativeLocation _defaultsceneroot))
  (bind _returnvalue_2 (+ _relativelocation (.location _returnvalue)))
  ;[1 1 1] Set_Click_Events
  (bind _asplayer_controller (Utilities|Casting|CastToPlayerController (Game|GetPlayerController 0)))
  (Variables|/Script/Engine.PlayerController|SetbEnableClickEvents _asplayer_controller true)
  (Variables|/Script/Engine.PlayerController|SetbEnableMouseOverEvents _asplayer_controller true)
  ;[1 1 1] UI dummys in Game?
  (if (Variables|Default|GetUI_Dummys_inGame?)
    (Development|SetHiddeninGame _icondummy_transform_2 false true)
    (else
      (Development|SetHiddeninGame _icondummy_transform_2 true true)))
  (if (Variables|Default|GetIcon_switch)
    ;[1 1 1] Set Billboard collsion
    (Collision|SetCollisionEnabled (Variables|Default|GetBox_Trigger) "QueryOnly")
    (else
      ;[1 1 1] set Billboard off and 3D on
      (Collision|SetCollisionEnabled (Variables|Default|GetBox_Trigger) "NoCollision")
      (Collision|SetCollisionEnabled (Variables|Default|GetClick_Highlight) "QueryOnly")
      ;[1 1 1] ZoomPoints_UI_scale and_position
      (Transformation|SetWorldRotation (Variables|Default|GetClickHighlight_Scale) (Variables|Default|GetButton_Rotation) false false)
      (Transformation|SetWorldScale3D (Variables|Default|GetClickHighlight_Scale) (Variables|/Script/Engine.SceneComponent|GetRelativeScale3D (Variables|Default|GetIconDummy_transform)))
      (Transformation|SetWorldLocation (Variables|Default|GetClickHighlight_Scale) _returnvalue_2 false false)
      (if (Variables|Default|GetTouch_Icon?)
        (Game|SpawnActorfromClass "/Game/Showroom_Navigation/UI/BP/BP_Touch_Icon.BP_Touch_Icon_C" (Math|Transform|MakeTransform _returnvalue_2 (Variables|Default|GetButton_Rotation) (Variables|/Script/Engine.SceneComponent|GetRelativeScale3D _icondummy_transform)) "AlwaysSpawn" 0 0)))))

(event EventTick
  (params (DeltaSeconds :type Float%20%28single-precision%29))
  ;[1 1 1] Text_Labels
  (if (Variables|Default|GetShowLabels)
    (Transformation|SetWorldRotation (Variables|Default|GetPivot) (Math|Rotator|FindLookatRotation (Transformation|GetActorLocation) (Transformation|GetActorLocation (Game|GetPlayerCameraManager 0))) false false)))

(fn ConstructionScript
  (bind _springarm (Variables|Default|GetSpringArm))
  (bind _icondummy_transform (Variables|Default|GetIconDummy_transform))
  ;[1 1 1] setup Camera
  (Transformation|SetRelativeRotation _springarm (Variables|Default|GetCamera_Rotation) false false)
  (Variables|/Script/Engine.SpringArmComponent|SetTargetArmLength _springarm (Variables|Default|GetZoomInPoint01Armlength))
  ;[1 1 1] Set FOV from Pawn
  (bind _returnvalue (Actor|GetActorOfClass "/Game/Showroom_Navigation/Blueprint/BP_MasterPawn.BP_MasterPawn_C"))
  (Camera|SetFieldOfView (Variables|Default|GetCamera) (Variables|/Game/Showroom_Navigation/Blueprint/BP_MasterPawn.BP_MasterPawn_C|GetField_of_View _returnvalue))
  ;[1 1 1] 3d Button transforms
  (Transformation|SetRelativeScale3D _icondummy_transform (Variables|Default|GetButton_Scale))
  (Transformation|SetRelativeLocation _icondummy_transform (Variables|Default|GetButton_Offset) false false)
  (Transformation|SetRelativeRotation _icondummy_transform (Variables|Default|GetButton_Rotation) false false)
  ;[1 1 1] Lock rotation
  (Transformation|SetWorldRotation (Variables|Default|GetDefaultSceneRoot) "0, 0, 0" false false)
  ;[1 1 1] construction Billboard
  (CallFunction|ConstructionBillboard)
  ;[1 1 1] PanoDummy_Set visibility
  (Rendering|SetVisibility (Variables|Default|GetPanoPoint) false false)
  (if (Variables|Default|GetPanoPoint_ON)
    (Rendering|SetVisibility (Variables|Default|GetPanoPoint) true false)
    ;[1 1 1] PanoDummy_set_Location
    (Transformation|SetWorldLocation (Variables|Default|GetPanoPoint) (+ (Variables|Default|GetPanoPointLocation) (Transformation|GetWorldLocation (Variables|Default|GetIconDummy_transform))) false false)))

(fn ConstructionBillboard
  (bind _billboard_size (Variables|Default|GetBillboard_size))
  (bind _text_size (Variables|Default|GetText_Size))
  (bind _onlytextsize (Variables|Default|GetOnlyTextSize))
  (bind _returnvalue (/ _billboard_size 32.0))
  (if (Variables|Default|GetIcon_switch)
    (Utilities|FlowControl|Sequence
      (:then_0
        ;[1 1 1] show Labels
        (if (Variables|Default|GetShowLabels)
          (Rendering|SetVisibility (Variables|Default|GetTextRender) true false)
          (else
            (Rendering|SetVisibility (Variables|Default|GetTextRender) false false))))
      (:then_1
        _))
    ;[1 1 1] set collisionens 3D of Billboard on
    (Rendering|SetVisibility (Variables|Default|GetBox_Trigger) true false)
    (Collision|SetCollisionEnabled (Variables|Default|GetBox_Trigger) "QueryOnly")
    (Collision|SetCollisionEnabled (Variables|Default|GetClick_Highlight) "NoCollision")
    ;[1 1 1] Set Billboard and Text Labeks
    (Class|MaterialBillboardComponent|SetElements (Variables|Default|GetMaterialBillboard) (Utilities|Array|MakeArray (Utilities|Struct|MakeMaterialSpriteElement (Variables|Default|GetBillboard_Material) 0 false _billboard_size _billboard_size)))
    (Rendering|Components|TextRender|SetText (Variables|Default|GetTextRender) (Utilities|Text|ToText(String) (Variables|Default|GetText%20Label)))
    ;[1 1 1] Billboard collider Button scale
    (Transformation|SetRelativeScale3D (Variables|Default|GetBox_Trigger) (Math|Vector|MakeVector _returnvalue _returnvalue _returnvalue))
    ;[1 1 1] Touch Icon OFF
    (Rendering|SetVisibility (Variables|Default|GetIconDummy_transform) false true)
    ;[1 1 1] Billboard offset
    (Transformation|SetRelativeLocation (Variables|Default|GetIcon_group) (Variables|Default|GetBillboard_Offset) false false)
    ;[1 1 1] Text Size and Offset
    (Transformation|SetRelativeScale3D _text_size (Math|Vector|MakeVector _onlytextsize _onlytextsize _onlytextsize))
    (Transformation|SetRelativeLocation _text_size (Math|Vector|MakeVector 0.0 (Variables|Default|GetTextOffset) 0.0) false false)
    (else
      ;[1 1 1] Set Billboard off
      (Rendering|SetVisibility (Variables|Default|GetBox_Trigger) false false)
      (Rendering|SetVisibility (Variables|Default|GetTextRender) false false))))

(fn TourButtonLabels
  (if (Variables|Default|GetActivate%20Tour%20Name)
    ;[1 1 1] Tour Names Enter Dialog
    (return (Variables|Default|GetTour%20Name))
    (else
      ;[1 1 1] TourNames from get DisplayName
      (return (Utilities|Text|ToText(String) (Utilities|String|Replace (Utilities|String|Replace (Utilities|String|Replace (Utilities|String|ToString(Text) (Utilities|Text|ToText(String) (Utilities|GetDisplayName self))) "BP_ZoomTarget") "BP_BaseTarget") "BP_WaypointTarget"))))))