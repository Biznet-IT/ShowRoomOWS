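; Clickable waypoint actor for showroom navigation, with its own camera, button and optional custom tour label.
; Click or non-drag touch stores its waypoint and tour indices in the GameInstance, calls the waypoint dispatcher and hides the button.
; MasterPawn overlap toggles the button, trigger collision and waypoint-tour flag.
; Construction script sets up camera arm, rotation, height and button placement, copying FOV from BP_MasterPawn.
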(event OnInputTouchEnd(Box_Trigger)
  (params (FingerIndex :type ETouchIndex%20Enum :default "Touch1") (TouchedComponent :type Primitive%20Component%20Object%20Reference))
  (bind _self self)
  ;[1 1 1] Do not open when Touch is moving
  (bind _asjumbo_owsgame_instance (Utilities|Casting|CastToJumboOWSGameInstance (Game|GetGameInstance)))
  (if (not (Variables|/Game/ThirdPersonBP/Blueprints/JumboOWSGameInstance.JumboOWSGameInstance_C|Getis_Touch_moving _asjumbo_owsgame_instance))
    ;[1 1 1] Find_this WayPoint in Array
    (bind _asjumbo_owsgame_instance_2 (Utilities|Casting|CastToJumboOWSGameInstance (Game|GetGameInstance)))
    (Variables|/Game/ThirdPersonBP/Blueprints/JumboOWSGameInstance.JumboOWSGameInstance_C|SetGI_GetWayP _asjumbo_owsgame_instance_2 (Utilities|Array|FindItem (Variables|/Game/ThirdPersonBP/Blueprints/JumboOWSGameInstance.JumboOWSGameInstance_C|GetWaypoint_Array _asjumbo_owsgame_instance_2) self))
    ;[1 1 1] Set Waypoint Tour Index
    (bind _asjumbo_owsgame_instance_3 (Utilities|Casting|CastToJumboOWSGameInstance (Game|GetGameInstance)))
    (if (Utilities|Array|ContainsItem (Variables|/Game/ThirdPersonBP/Blueprints/JumboOWSGameInstance.JumboOWSGameInstance_C|GetGI_TourArray _asjumbo_owsgame_instance_3) _self)
      (Variables|/Game/ThirdPersonBP/Blueprints/JumboOWSGameInstance.JumboOWSGameInstance_C|SetGI_Tour_Button_index _asjumbo_owsgame_instance_3 (Utilities|Array|FindItem (Variables|/Game/ThirdPersonBP/Blueprints/JumboOWSGameInstance.JumboOWSGameInstance_C|GetGI_TourArray _asjumbo_owsgame_instance_3) _self))
      (else
        (Variables|/Game/ThirdPersonBP/Blueprints/JumboOWSGameInstance.JumboOWSGameInstance_C|SetGI_Tour_Button_index _asjumbo_owsgame_instance_3 -500)))
    (Default|CallEventDispatcherWaypoint)
    (Rendering|SetVisibility (Variables|Default|GetButton) false true)))

(event OnClicked(Box_Trigger)
  (params (TouchedComponent :type Primitive%20Component%20Object%20Reference) (ButtonPressed :type Key%20Structure :default "None"))
  (bind _self self)
  ;[1 1 1] Do not open when Touch is moving
  (bind _asjumbo_owsgame_instance (Utilities|Casting|CastToJumboOWSGameInstance (Game|GetGameInstance)))
  (if (not (Variables|/Game/ThirdPersonBP/Blueprints/JumboOWSGameInstance.JumboOWSGameInstance_C|Getis%20first%20touch _asjumbo_owsgame_instance))
    ;[1 1 1] Find_this WayPoint in Array
    (bind _asjumbo_owsgame_instance_2 (Utilities|Casting|CastToJumboOWSGameInstance (Game|GetGameInstance)))
    (Variables|/Game/ThirdPersonBP/Blueprints/JumboOWSGameInstance.JumboOWSGameInstance_C|SetGI_GetWayP _asjumbo_owsgame_instance_2 (Utilities|Array|FindItem (Variables|/Game/ThirdPersonBP/Blueprints/JumboOWSGameInstance.JumboOWSGameInstance_C|GetWaypoint_Array _asjumbo_owsgame_instance_2) self))
    ;[1 1 1] Set Waypoint Tour Index
    (bind _asjumbo_owsgame_instance_3 (Utilities|Casting|CastToJumboOWSGameInstance (Game|GetGameInstance)))
    (if (Utilities|Array|ContainsItem (Variables|/Game/ThirdPersonBP/Blueprints/JumboOWSGameInstance.JumboOWSGameInstance_C|GetGI_TourArray _asjumbo_owsgame_instance_3) _self)
      (Variables|/Game/ThirdPersonBP/Blueprints/JumboOWSGameInstance.JumboOWSGameInstance_C|SetGI_Tour_Button_index _asjumbo_owsgame_instance_3 (Utilities|Array|FindItem (Variables|/Game/ThirdPersonBP/Blueprints/JumboOWSGameInstance.JumboOWSGameInstance_C|GetGI_TourArray _asjumbo_owsgame_instance_3) _self))
      (else
        (Variables|/Game/ThirdPersonBP/Blueprints/JumboOWSGameInstance.JumboOWSGameInstance_C|SetGI_Tour_Button_index _asjumbo_owsgame_instance_3 -500)))
    (Default|CallEventDispatcherWaypoint)
    (Rendering|SetVisibility (Variables|Default|GetButton) false true)))

(event OnComponentEndOverlap(Box_Trigger_1)
  (params (OverlappedComponent :type Primitive%20Component%20Object%20Reference) (OtherActor :type Actor%20Object%20Reference) (OtherComp :type Primitive%20Component%20Object%20Reference) (OtherBodyIndex :type Integer))
  (if (Actor|ActorHasTag OtherActor "MasterPawn")
    ;[1 1 1] Set Waypoint on/off when Pawn enters
    (Rendering|SetVisibility (Variables|Default|GetButton) true true)
    (Collision|SetCollisionEnabled (Variables|Default|GetBox_Trigger) "QueryOnly")
    (bind _asjumbo_owsgame_instance (Utilities|Casting|CastToJumboOWSGameInstance (Game|GetGameInstance)))
    (Variables|/Game/ThirdPersonBP/Blueprints/JumboOWSGameInstance.JumboOWSGameInstance_C|SetGI_is_waypointTour _asjumbo_owsgame_instance false)))

(event OnComponentBeginOverlap(Box_Trigger_1)
  (params (OverlappedComponent :type Primitive%20Component%20Object%20Reference) (OtherActor :type Actor%20Object%20Reference) (OtherComp :type Primitive%20Component%20Object%20Reference) (OtherBodyIndex :type Integer) (bFromSweep :type Boolean) (SweepResult :type Hit%20Result%20Structure%20%28by%20ref%29))
  (if (Actor|ActorHasTag OtherActor "MasterPawn")
    ;[1 1 1] Set Waypoint on/off when Pawn enters
    (Rendering|SetVisibility (Variables|Default|GetButton) false true)
    (Collision|SetCollisionEnabled (Variables|Default|GetBox_Trigger) "NoCollision")
    (bind _asjumbo_owsgame_instance (Utilities|Casting|CastToJumboOWSGameInstance (Game|GetGameInstance)))
    (Variables|/Game/ThirdPersonBP/Blueprints/JumboOWSGameInstance.JumboOWSGameInstance_C|SetGI_is_waypointTour _asjumbo_owsgame_instance true)))

(fn ConstructionScript
  (bind _transform_dummy (Variables|Default|GetTransform_dummy))
  (bind _returnvalue (Transformation|GetWorldLocation _transform_dummy))
  ;[1 1 1] Set sspringarm 0
  (Variables|/Script/Engine.SpringArmComponent|SetTargetArmLength (Variables|Default|GetSpringArm) (Variables|Default|GetWaypointArmLength))
  ;[1 1 1] Set FOV from Pawn
  (bind _returnvalue_2 (Actor|GetActorOfClass "/Game/Showroom_Navigation/Blueprint/BP_MasterPawn.BP_MasterPawn_C"))
  (Camera|SetFieldOfView (Variables|Default|GetCamera) (Variables|/Game/Showroom_Navigation/Blueprint/BP_MasterPawn.BP_MasterPawn_C|GetField_of_View _returnvalue_2))
  ;[1 1 1] Camera height Offset
  (Transformation|AddLocalOffset (Variables|Default|GetSpringArm) (Math|Vector|MakeVector 0.0 0.0 (Variables|Default|Getset_Camera_height_Offset)) false false)
  ;[1 1 1] Set Waypoint Transforms
  (Transformation|SetWorldLocation (Variables|Default|GetButton) (+ (Variables|/Script/Engine.SceneComponent|GetRelativeLocation (Variables|Default|GetDefaultSceneRoot1)) (Variables|Default|GetIcon_Offset)) false false)
  (Transformation|SetWorldLocation _transform_dummy (Math|Vector|MakeVector (.x _returnvalue) (.y _returnvalue) (.z (Transformation|GetWorldLocation (Variables|Default|GetBox_Trigger)))) false false)
  (Transformation|SetWorldScale3D (Variables|Default|GetButton) (Variables|Default|GetButton_Scale))
  (Transformation|SetWorldRotation (Variables|Default|GetPointer_center) (Variables|Default|GetWaypoint_Cam_Rotation) false false))

(fn TourButtonLabels
  (if (Variables|Default|GetActivate%20Tour%20Name)
    ;[1 1 1] TourName_Enter_Dialog
    (return (Variables|Default|GetTour%20Name))
    (else
      ;[1 1 1] TourName Enter Display Names
      (return (Utilities|Text|ToText(String) (Utilities|String|Replace (Utilities|String|Replace (Utilities|String|Replace (Utilities|String|ToString(Text) (Utilities|Text|ToText(String) (Utilities|GetDisplayName self))) "BP_ZoomTarget") "BP_BaseTarget") "BP_WaypointTarget"))))))