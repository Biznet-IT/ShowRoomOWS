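; BP_Crosshair is a world-space focus marker for the cinematic camera, BP_Cine_Camera.
; On Tick it moves its mesh to the camera's FocusLoc, mirrors UIVisible, and branches on FocusSetting to destroy itself or face the camera, continuously or once.
; In the last mode it locks a world-space offset from the camera and writes the resulting point back to FocusLoc.
; Reset re-arms the one-time steps.
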(event Custom|Reset
  (Utilities|FlowControl|Sequence
    (:then_0
      (Utilities|FlowControl|DoOnce false) ; enters at Reset
    )
    (:then_1
      (Utilities|FlowControl|DoOnce false) ; enters at Reset
    )))

(event EventTick
  (params (DeltaSeconds :type Float%20%28single-precision%29))
  (bind _staticmeshcomponent (Variables|Debug|GetStaticMeshComponent))
  (bind _cinematicspectator_ref (Variables|Default|GetCinematicSpectator%20Ref))
  (bind _staticmeshcomponent_2 (Variables|Debug|GetStaticMeshComponent))
  (bind _returnvalue (Transformation|GetWorldLocation _staticmeshcomponent_2))
  (bind _cinecamera (Variables|/Game/Cine_Cam/BP_Cine_Camera.BP_Cine_Camera_C|GetCineCamera _cinematicspectator_ref))
  (bind _returnvalue_2 (Transformation|GetWorldLocation _cinecamera))
  (bind _returnvalue_3 (- _returnvalue_2 _returnvalue))
  (Transformation|SetWorldLocation (Variables|Debug|GetStaticMeshComponent) (Variables|/Game/Cine_Cam/BP_Cine_Camera.BP_Cine_Camera_C|GetFocusLoc (Variables|Default|GetCinematicSpectator%20Ref)) false false)
  (if (Variables|/Game/Cine_Cam/BP_Cine_Camera.BP_Cine_Camera_C|GetUI%20Visible? (Variables|Default|GetCinematicSpectator%20Ref))
    (Rendering|SetVisibility _staticmeshcomponent true false)
    (else
      (Rendering|SetVisibility _staticmeshcomponent false false)))
  (switch int (Variables|/Game/Cine_Cam/BP_Cine_Camera.BP_Cine_Camera_C|GetFocus%20Setting (Variables|Default|GetCinematicSpectator%20Ref))
    (:0
      (Actor|DestroyActor))
    (:1
      (Transformation|SetWorldRotation (Variables|Debug|GetStaticMeshComponent) (Math|Rotator|FindLookatRotation (Transformation|GetActorLocation) (Transformation|GetWorldLocation (Variables|/Game/Cine_Cam/BP_Cine_Camera.BP_Cine_Camera_C|GetCineCamera (Variables|Default|GetCinematicSpectator%20Ref)))) false false :!label _label))
    (:2
      (Variables|Default|SetVDelta _returnvalue_3)
      (Utilities|FlowControl|DoOnce false
        (:Completed
          (goto _label))))
    (:3
      (Utilities|FlowControl|Sequence
        (:then_0
          (Utilities|FlowControl|DoOnce false
            (:Completed
              (Variables|Default|SetVDelta _returnvalue_3)
              (goto _label))))
        (:then_1
          (Transformation|SetWorldLocation (Variables|Debug|GetStaticMeshComponent) (- _returnvalue_2 (Variables|Default|GetVDelta)) false false)
          (Variables|/Game/Cine_Cam/BP_Cine_Camera.BP_Cine_Camera_C|SetFocusLoc (Variables|Default|GetCinematicSpectator%20Ref) (- _returnvalue_2 (Variables|Default|GetVDelta))))))))

(event EventBeginPlay
  (bind _asbp_cine_camera (Utilities|Casting|CastToBP_Cine_Camera (Game|GetPlayerCharacter 0)))
  (Variables|Default|SetCinematicSpectator%20Ref _asbp_cine_camera))

(fn ConstructionScript)